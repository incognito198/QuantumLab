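; BP_Interferometer builds the socket board for an interferometer setup with laser, photo-detector, mirror and target parts.
; On BeginPlay it spawns a SizeX by SizeY grid of BP_Socket actors from its own location, storing each one's array index on the socket.
; It then sets the expected TargetActor on specific hard-coded socket indices, so the layout depends on grid dimensions.
; InetferometreAssembleState and Object are empty stubs.
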(event EventBeginPlay
  (bind _targetphotodel (Variables|Default|GetTargetPhotodel))
  (bind _targetmirror (Variables|Default|GetTargetMirror))
  (Utilities|FlowControl|Sequence
    (:then_0
      (for _index (range 0 (- (Variables|Default|GetsizeX) 1))
        (for _index_2 (range 0 (- (Variables|Default|GetsizeY) 1))
          (bind _returnvalue (Game|SpawnActorfromClass "/Game/CustomLogic/BP_Socket.BP_Socket_C" (Math|Conversions|ToTransform(Vector) (+ (Math|Vector|MakeVector (* _index (Variables|Default|GetSocketSpacing)) (* _index_2 (Variables|Default|GetSocketSpacing)) 0.0) (Transformation|GetActorLocation))) "Undefined" self 0))
          (bind _returnvalue_2 (Utilities|Array|Add (Variables|Default|GetSockets) _returnvalue))
          (Variables|/Game/CustomLogic/BP_Socket.BP_Socket_C|SetSocetIndex _returnvalue _returnvalue_2))))
    (:then_1
      (for (_array_element _array_index) (Variables|Default|GetSockets)
        (Utilities|FlowControl|Sequence
          (:then_0
            (if (== _array_index 502)
              (Variables|/Game/CustomLogic/BP_Socket.BP_Socket_C|SetTargetActor _array_element (Variables|Default|GetTargetLaser))))
          (:then_1
            (if (== _array_index 495)
              (Variables|/Game/CustomLogic/BP_Socket.BP_Socket_C|SetTargetActor _array_element _targetphotodel)))
          (:then_2
            (if (== _array_index 90)
              (Variables|/Game/CustomLogic/BP_Socket.BP_Socket_C|SetTargetActor _array_element _targetphotodel)))
          (:then_3
            (if (== _array_index 480)
              (Variables|/Game/CustomLogic/BP_Socket.BP_Socket_C|SetTargetActor _array_element _targetmirror)))
          (:then_4
            (if (== _array_index 105)
              (Variables|/Game/CustomLogic/BP_Socket.BP_Socket_C|SetTargetActor _array_element _targetmirror)))
          (:then_5
            (if (== _array_index 81)
              (Variables|/Game/CustomLogic/BP_Socket.BP_Socket_C|SetTargetActor _array_element (Variables|Default|GetTargetMishen)))))))))

(fn ConstructionScript)

(fn InetferometreAssembleState
  (return))

(fn Object
  (params (ObjectIn :type Actor%20Object%20Reference)))