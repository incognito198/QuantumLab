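; Clickable socket actor that spawns interferometer components, such as a laser, mirror, photodetector or target, at its location.
; Object stores the passed object's class; controller, touch or cube clicks spawn it if it matches TargetActor and the socket is inactive, then mark it active and apply per-class rotation.
; Cube clicks also pass the socket to all InterferometrMove interface actors.
; InetferometreAssembleState is empty, and socket-index checks remain unwired.
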(event OnClicked(Cube)
  (params (TouchedComponent :type Primitive%20Component%20Object%20Reference) (ButtonPressed :type Key%20Structure :default "None"))
  (bind _class (Variables|Default|GetClass))
  (Utilities|FlowControl|Sequence
    (:then_0
      (if (not (Variables|Default|GetIsActive))
        (Development|PrintString (Utilities|String|ToString(Integer) (Variables|Default|GetSocetIndex)))
        (if (== (Variables|Default|GetTargetActor) _class)
          (bind _returnvalue (Game|SpawnActorfromClass _class (Math|Conversions|ToTransform(Vector) (Transformation|GetActorLocation)) "Undefined" 0 0))
          (Variables|Default|SetIsActive true)
          (Utilities|FlowControl|Sequence
            (:then_0
              (if (== (Variables|Default|GetClass) "/Game/CustomLogic/BP_Interferometer/BP_Komponenti/Laser/BP_Laser.BP_Laser_C")
                (Class|Actor|AddActorWorldRotation _returnvalue "0,180.000000, 0")
                (Actor|GetAllActorsOfClass "BP_Socket_C")))
            (:then_1
              (if (== (Variables|Default|GetClass) "/Game/CustomLogic/BP_Interferometer/BP_Komponenti/Mirror/BP_Mirror.BP_Mirror_C")
                (Class|Actor|AddActorWorldRotation _returnvalue "0,-45.000000, 0")))
            (:then_2
              (if (== (Variables|Default|GetClass) "/Game/CustomLogic/BP_Interferometer/BP_Komponenti/BP_PhotodelBaseCopy.BP_PhotodelBaseCopy_C")
                (Class|Actor|AddActorWorldRotation _returnvalue "0,-45.000000, 0")))
            (:then_3
              (if (== (Variables|Default|GetClass) "/Game/CustomLogic/BP_Interferometer/BP_Komponenti/Mishen/BP_Mishen.BP_Mishen_C")
                (Class|Actor|AddActorWorldRotation _returnvalue "0,180.000000, 0")))))))
    (:then_1
      (bind _outactors (Actor|GetAllActorswithInterface "/Game/CustomLogic/BP_Interferometer/InterferometrMove.InterferometrMove_C"))
      (Class|InterferometrMove|MoveInterferometr(Message) _outactors self))))

(event Custom|HandleControllerClick
  (bind _class (Variables|Default|GetClass))
  (if (not (Variables|Default|GetIsActive))
    (Development|PrintString (Utilities|String|ToString(Integer) (Variables|Default|GetSocetIndex)))
    (if (== (Variables|Default|GetTargetActor) _class)
      (bind _returnvalue (Game|SpawnActorfromClass _class (Math|Conversions|ToTransform(Vector) (Transformation|GetActorLocation)) "Undefined" 0 0))
      (Variables|Default|SetIsActive true)
      (Utilities|FlowControl|Sequence
        (:then_0
          (if (== (Variables|Default|GetClass) "/Game/CustomLogic/BP_Interferometer/BP_Komponenti/Laser/BP_Laser.BP_Laser_C")
            (Class|Actor|AddActorWorldRotation _returnvalue "0,180.000000, 0")
            (Actor|GetAllActorsOfClass "BP_Socket_C")))
        (:then_1
          (if (== (Variables|Default|GetClass) "/Game/CustomLogic/BP_Interferometer/BP_Komponenti/Mirror/BP_Mirror.BP_Mirror_C")
            (Class|Actor|AddActorWorldRotation _returnvalue "0,-45.000000, 0")))
        (:then_2
          (if (== (Variables|Default|GetClass) "/Game/CustomLogic/BP_Interferometer/BP_Komponenti/BP_PhotodelBaseCopy.BP_PhotodelBaseCopy_C")
            (Class|Actor|AddActorWorldRotation _returnvalue "0,-45.000000, 0")))
        (:then_3
          (if (== (Variables|Default|GetClass) "/Game/CustomLogic/BP_Interferometer/BP_Komponenti/Mishen/BP_Mishen.BP_Mishen_C")
            (Class|Actor|AddActorWorldRotation _returnvalue "0,180.000000, 0")))))))

(event EventActorOnInputTouchBegin
  (params (FingerIndex :type ETouchIndex%20Enum :default "Touch1"))
  (bind _class (Variables|Default|GetClass))
  (if (not (Variables|Default|GetIsActive))
    (Development|PrintString (Utilities|String|ToString(Integer) (Variables|Default|GetSocetIndex)))
    (if (== (Variables|Default|GetTargetActor) _class)
      (bind _returnvalue (Game|SpawnActorfromClass _class (Math|Conversions|ToTransform(Vector) (Transformation|GetActorLocation)) "Undefined" 0 0))
      (Variables|Default|SetIsActive true)
      (Utilities|FlowControl|Sequence
        (:then_0
          (if (== (Variables|Default|GetClass) "/Game/CustomLogic/BP_Interferometer/BP_Komponenti/Laser/BP_Laser.BP_Laser_C")
            (Class|Actor|AddActorWorldRotation _returnvalue "0,180.000000, 0")
            (Actor|GetAllActorsOfClass "BP_Socket_C")))
        (:then_1
          (if (== (Variables|Default|GetClass) "/Game/CustomLogic/BP_Interferometer/BP_Komponenti/Mirror/BP_Mirror.BP_Mirror_C")
            (Class|Actor|AddActorWorldRotation _returnvalue "0,-45.000000, 0")))
        (:then_2
          (if (== (Variables|Default|GetClass) "/Game/CustomLogic/BP_Interferometer/BP_Komponenti/BP_PhotodelBaseCopy.BP_PhotodelBaseCopy_C")
            (Class|Actor|AddActorWorldRotation _returnvalue "0,-45.000000, 0")))
        (:then_3
          (if (== (Variables|Default|GetClass) "/Game/CustomLogic/BP_Interferometer/BP_Komponenti/Mishen/BP_Mishen.BP_Mishen_C")
            (Class|Actor|AddActorWorldRotation _returnvalue "0,180.000000, 0")))))))

(fn ConstructionScript)

(fn InetferometreAssembleState
  (return))

(fn Object
  (params (ObjectIn :type Actor%20Object%20Reference))
  (Variables|Default|SetClass (Utilities|GetClass ObjectIn))
  (return 0))