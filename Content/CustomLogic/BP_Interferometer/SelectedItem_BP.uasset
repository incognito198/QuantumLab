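; SelectedItem_BP tracks the currently selected item in the interferometer logic and can destroy it on request.
; SelectItem stores the item, then sends MirrorMessage or ScrewMessage to all HighlightInserted_Interface actors, depending on whether it is a mirror or screw.
; DestroyItem destroys a selected mirror or screw and clears the reference.
; The BP_Photodel branch is empty, the trailing delay leads nowhere, and the UnselectMessage call is unconnected.
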(event EventSelectItem
  (params (NewParam :type Inserted%20Idems%20Parent%20BP%20Object%20Reference))
  (bind _output_get (Variables|Default|SetSelectedItem NewParam))
  (bind _outactors (Actor|GetAllActorswithInterface "/Game/CustomLogic/BP_Interferometer/InsertedItems/HighlightInserted_Interface.HighlightInserted_Interface_C"))
  (Utilities|FlowControl|Sequence
    (:then_0
      (Utilities|Casting|CastToMirror_BP _output_get)
      (Class|HighlightInsertedInterface|Mirror(Message) _outactors)
      (Utilities|FlowControl|Delay 5.0 :!label _label))
    (:then_1
      (Utilities|Casting|CastToScrew_BP _output_get)
      (Class|HighlightInsertedInterface|Screw(Message) _outactors)
      (goto _label))
    (:then_2
      (Utilities|Casting|CastToBP_Photodel _output_get))))

(event EventDestroyItem
  (Utilities|FlowControl|Sequence
    (:then_0
      (bind _asmirror_bp (Utilities|Casting|CastToMirror_BP (Variables|Default|GetSelectedItem)))
      (Actor|DestroyActor _asmirror_bp))
    (:then_1
      (bind _asscrew_bp (Utilities|Casting|CastToScrew_BP (Variables|Default|GetSelectedItem)))
      (Actor|DestroyActor _asscrew_bp)))
  (Variables|Default|SetSelectedItem 0))

(fn ConstructionScript)