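; Copy of the interferometer's "Photodel" base that mirrors the finished assembly of an original.
; When OriginalAssembleComplete receives success, AssembleCheck reveals the stand, clamps, screws, micrometer screw and lens meshes.
; KomponentToAdd only records the class of the passed part.
; The AssembleState camera-blend and transform logic, along with the per-part completion check, is disconnected and never runs.
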(event Custom|AssembleCheck
  (Rendering|SetVisibility (Variables|Default|GetСМ_Зажим2) true false))

(event Collision|EventActorBeginOverlap
  (params (OtherActor :type Actor%20Object%20Reference))
  (|CallParentFunction OtherActor) ; This node is disabled and will not be called.\nDrag off pins to build functionality.
)

(fn ConstructionScript
  (|CallParentFunction))

(fn KomponenttoAdd
  (params (ObjectIn :type Actor%20Object%20Reference))
  (Variables|Default|SetPhotodelPart (Utilities|GetClass ObjectIn))
  (return 0))

(fn AssembleState
  (params (AssembleStarted? :type Boolean) (AssembleEnded? :type Boolean)))

(fn OriginalAssembleComplete
  (params (OriginalAssembleComplite :type Boolean))
  (bind _output_get (Variables|Default|SetAssemble%20Success? OriginalAssembleComplite))
  (if _output_get
    (CallFunction|AssembleCheck)
    (return false)))