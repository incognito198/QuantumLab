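; Base actor for the interferometer's Photodel unit, a click-to-assemble puzzle that opens an assembly widget.
; AssembleState blends to another camera and moves the actor to a fixed enlarged pose, or restores both.
; Each of seven click zones requires a tagged part actor in the world, then reveals and timeline-animates its mesh.
; Completion notifies copies through BPI_PhotodelCopyAssemble and reshows the widget; BeginPlay copies completion state from the first instance.
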(event OnClicked(ObjectToSpawn)
  (params (TouchedComponent :type Primitive%20Component%20Object%20Reference) (ButtonPressed :type Key%20Structure))
  (bind _widjet (Variables|Default|GetWidjet))
  (if (not (Variables|Default|GetAssembleComplite?))
    (if (not (UserInterface|Viewport|IsinViewport _widjet))
      (if (and (Variables|Default|GetAssemble%20Started?) (not (Variables|Default|GetAssembleComplite?)))
        (Development|PrintString "Сборка не завершена!" true true "(R=1.000000,G=0.012904,B=0.000000,A=1.000000)" 3.0)
        (else
          (UserInterface|Viewport|AddtoViewport _widjet 0))))))

(event OnClicked(TZ_Zazhim1)
  (params (TouchedComponent :type Primitive%20Component%20Object%20Reference) (ButtonPressed :type Key%20Structure))
  (bind _см_зажим1 (Variables|Default|GetСМ_Зажим1))
  (bind _relativelocation (Variables|/Script/Engine.SceneComponent|GetRelativeLocation _см_зажим1))
  (bind _outactors (Actor|GetAllActorsOfClasswithTag (Variables|Default|GetPhotodelPart) "3"))
  (if (Utilities|Array|IsValidIndex _outactors)
    (if (not (Variables|Default|GetZazhim1IsActive?))
      (Variables|Default|SetZazhim1IsActive? true)
      (Rendering|SetVisibility (Variables|Default|GetСМ_Зажим1) true false)
      (bind _y (Timeline|Zazh1 PlayFromStart)
        (:Update
          (Transformation|SetRelativeLocation _см_зажим1 (Math|Vector|MakeVector (.x _relativelocation) _y (.z _relativelocation)) false true)
          (bind _output_get (Variables|Default|SetAssembleComplite? (Math|Boolean|ANDBoolean (Variables|Default|GetStojkaIsActive?) (Variables|Default|GetZazhim1IsActive?) (Variables|Default|GetZazhim2IsActive?) (Variables|Default|GetLenseIsActive?) (Variables|Default|GetBolt1IsActive?) (Variables|Default|GetBolt2IsActive?) (Variables|Default|GetMicrVintIsActive?))))
          (if _output_get
            (bind _outactors_2 (Actor|GetAllActorswithInterface "/Game/CustomLogic/BP_Interferometer/BP_Komponenti/BPI_PhotodelCopyAssemble.BPI_PhotodelCopyAssemble_C"))
            (Class|BPIPhotodelCopyAssemble|OriginalAssembleComplete(Message) _outactors_2 (Math|Boolean|ANDBoolean (Variables|Default|GetStojkaIsActive?) (Variables|Default|GetZazhim1IsActive?) (Variables|Default|GetZazhim2IsActive?) (Variables|Default|GetLenseIsActive?) (Variables|Default|GetBolt1IsActive?) (Variables|Default|GetBolt2IsActive?) (Variables|Default|GetMicrVintIsActive?)))
            (Utilities|FlowControl|Delay 2.0)
            (CallFunction|AssembleCheck)
            (UserInterface|Viewport|AddtoViewport (Variables|Default|GetWidjet) 0)))
        (:Finished
          (Development|PrintString "Пятка установлена"))))))

(event OnClicked(TZ_Zazhim2)
  (params (TouchedComponent :type Primitive%20Component%20Object%20Reference) (ButtonPressed :type Key%20Structure))
  (bind _см_зажим2 (Variables|Default|GetСМ_Зажим2))
  (bind _relativelocation (Variables|/Script/Engine.SceneComponent|GetRelativeLocation _см_зажим2))
  (bind _outactors (Actor|GetAllActorsOfClasswithTag (Variables|Default|GetPhotodelPart) "2"))
  (if (Utilities|Array|IsValidIndex _outactors)
    (if (not (Variables|Default|GetZazhim2IsActive?))
      (Variables|Default|SetZazhim2IsActive? true)
      (Rendering|SetVisibility (Variables|Default|GetСМ_Зажим2) true false)
      (bind _z (Timeline|Zazh2 PlayFromStart)
        (:Update
          (Transformation|SetRelativeLocation _см_зажим2 (Math|Vector|MakeVector (.x _relativelocation) (.y _relativelocation) _z) false true)
          (Development|PrintString "зажим установлен")
          (bind _output_get (Variables|Default|SetAssembleComplite? (Math|Boolean|ANDBoolean (Variables|Default|GetStojkaIsActive?) (Variables|Default|GetZazhim1IsActive?) (Variables|Default|GetZazhim2IsActive?) (Variables|Default|GetLenseIsActive?) (Variables|Default|GetBolt1IsActive?) (Variables|Default|GetBolt2IsActive?) (Variables|Default|GetMicrVintIsActive?))))
          (if _output_get
            (bind _outactors_2 (Actor|GetAllActorswithInterface "/Game/CustomLogic/BP_Interferometer/BP_Komponenti/BPI_PhotodelCopyAssemble.BPI_PhotodelCopyAssemble_C"))
            (Class|BPIPhotodelCopyAssemble|OriginalAssembleComplete(Message) _outactors_2 (Math|Boolean|ANDBoolean (Variables|Default|GetStojkaIsActive?) (Variables|Default|GetZazhim1IsActive?) (Variables|Default|GetZazhim2IsActive?) (Variables|Default|GetLenseIsActive?) (Variables|Default|GetBolt1IsActive?) (Variables|Default|GetBolt2IsActive?) (Variables|Default|GetMicrVintIsActive?)))
            (Utilities|FlowControl|Delay 2.0)
            (CallFunction|AssembleCheck)
            (UserInterface|Viewport|AddtoViewport (Variables|Default|GetWidjet) 0)))))))

(event OnClicked(TZ_MicrVint)
  (params (TouchedComponent :type Primitive%20Component%20Object%20Reference) (ButtonPressed :type Key%20Structure))
  (bind _см_микрвинт (Variables|Default|GetСМ_МикрВинт))
  (bind _relativelocation (Variables|/Script/Engine.SceneComponent|GetRelativeLocation _см_микрвинт))
  (bind _relativerotation (Variables|/Script/Engine.SceneComponent|GetRelativeRotation _см_микрвинт))
  (bind _outactors (Actor|GetAllActorsOfClasswithTag (Variables|Default|GetPhotodelPart) "7"))
  (if (Utilities|Array|IsValidIndex _outactors)
    (if (not (Variables|Default|GetMicrVintIsActive?))
      (Variables|Default|SetMicrVintIsActive? true)
      (Rendering|SetVisibility (Variables|Default|GetСМ_МикрВинт) true false)
      (bind (_direction _y _yrot) (Timeline|Micr PlayFromStart)
        (:Update
          (Transformation|SetRelativeLocationAndRotation _см_микрвинт (Math|Vector|MakeVector (.x _relativelocation) _y (.z _relativelocation)) (Math|Rotator|MakeRotator (.roll _relativerotation) _yrot (.yaw _relativerotation)) false false)
          (Development|PrintString "Микрометрический винт установлен")
          (bind _output_get (Variables|Default|SetAssembleComplite? (Math|Boolean|ANDBoolean (Variables|Default|GetStojkaIsActive?) (Variables|Default|GetZazhim1IsActive?) (Variables|Default|GetZazhim2IsActive?) (Variables|Default|GetLenseIsActive?) (Variables|Default|GetBolt1IsActive?) (Variables|Default|GetBolt2IsActive?) (Variables|Default|GetMicrVintIsActive?))))
          (if _output_get
            (bind _outactors_2 (Actor|GetAllActorswithInterface "/Game/CustomLogic/BP_Interferometer/BP_Komponenti/BPI_PhotodelCopyAssemble.BPI_PhotodelCopyAssemble_C"))
            (Class|BPIPhotodelCopyAssemble|OriginalAssembleComplete(Message) _outactors_2 (Math|Boolean|ANDBoolean (Variables|Default|GetStojkaIsActive?) (Variables|Default|GetZazhim1IsActive?) (Variables|Default|GetZazhim2IsActive?) (Variables|Default|GetLenseIsActive?) (Variables|Default|GetBolt1IsActive?) (Variables|Default|GetBolt2IsActive?) (Variables|Default|GetMicrVintIsActive?)))
            (Utilities|FlowControl|Delay 2.0)
            (CallFunction|AssembleCheck)
            (UserInterface|Viewport|AddtoViewport (Variables|Default|GetWidjet) 0)))))))

(event OnClicked(TZ_Vint1)
  (params (TouchedComponent :type Primitive%20Component%20Object%20Reference) (ButtonPressed :type Key%20Structure))
  (bind _см_винт1 (Variables|Default|GetСМ_Винт1))
  (bind _relativelocation (Variables|/Script/Engine.SceneComponent|GetRelativeLocation _см_винт1))
  (bind _outactors (Actor|GetAllActorsOfClasswithTag (Variables|Default|GetPhotodelPart) "5"))
  (if (Utilities|Array|IsValidIndex _outactors)
    (if (not (Variables|Default|GetBolt1IsActive?))
      (Variables|Default|SetBolt1IsActive? true)
      (Rendering|SetVisibility (Variables|Default|GetСМ_Винт1) true false)
      (bind (_direction _y _yrot) (Timeline|Vint1 PlayFromStart)
        (:Update
          (Transformation|SetRelativeLocationAndRotation _см_винт1 (Math|Vector|MakeVector (.x _relativelocation) _y (.z _relativelocation)) (Math|Rotator|MakeRotator 0.0 _yrot 0.0) false false)
          (Development|PrintString "Винт 1 установлен")
          (bind _output_get (Variables|Default|SetAssembleComplite? (Math|Boolean|ANDBoolean (Variables|Default|GetStojkaIsActive?) (Variables|Default|GetZazhim1IsActive?) (Variables|Default|GetZazhim2IsActive?) (Variables|Default|GetLenseIsActive?) (Variables|Default|GetBolt1IsActive?) (Variables|Default|GetBolt2IsActive?) (Variables|Default|GetMicrVintIsActive?))))
          (if _output_get
            (bind _outactors_2 (Actor|GetAllActorswithInterface "/Game/CustomLogic/BP_Interferometer/BP_Komponenti/BPI_PhotodelCopyAssemble.BPI_PhotodelCopyAssemble_C"))
            (Class|BPIPhotodelCopyAssemble|OriginalAssembleComplete(Message) _outactors_2 (Math|Boolean|ANDBoolean (Variables|Default|GetStojkaIsActive?) (Variables|Default|GetZazhim1IsActive?) (Variables|Default|GetZazhim2IsActive?) (Variables|Default|GetLenseIsActive?) (Variables|Default|GetBolt1IsActive?) (Variables|Default|GetBolt2IsActive?) (Variables|Default|GetMicrVintIsActive?)))
            (Utilities|FlowControl|Delay 2.0)
            (CallFunction|AssembleCheck)
            (UserInterface|Viewport|AddtoViewport (Variables|Default|GetWidjet) 0)))))))

(event OnClicked(TZ_Lense)
  (params (TouchedComponent :type Primitive%20Component%20Object%20Reference) (ButtonPressed :type Key%20Structure))
  (bind _см_линза (Variables|Default|GetСМ_Линза))
  (bind _relativerotation (Variables|/Script/Engine.SceneComponent|GetRelativeRotation _см_линза))
  (bind _outactors (Actor|GetAllActorsOfClasswithTag (Variables|Default|GetPhotodelPart) "6"))
  (if (Utilities|Array|IsValidIndex _outactors)
    (if (not (Variables|Default|GetLenseIsActive?))
      (Variables|Default|SetLenseIsActive? true)
      (Rendering|SetVisibility (Variables|Default|GetСМ_Линза) true false)
      (bind (_direction _z _x _yrot) (Timeline|Lense PlayFromStart)
        (:Update
          (Transformation|SetRelativeLocationAndRotation _см_линза (Math|Vector|MakeVector _x (.y (Variables|/Script/Engine.SceneComponent|GetRelativeLocation _см_линза)) _z) (Math|Rotator|MakeRotator (.roll _relativerotation) _yrot (.yaw _relativerotation)) false false)
          (Development|PrintString "Линза установлена")
          (bind _output_get (Variables|Default|SetAssembleComplite? (Math|Boolean|ANDBoolean (Variables|Default|GetStojkaIsActive?) (Variables|Default|GetZazhim1IsActive?) (Variables|Default|GetZazhim2IsActive?) (Variables|Default|GetLenseIsActive?) (Variables|Default|GetBolt1IsActive?) (Variables|Default|GetBolt2IsActive?) (Variables|Default|GetMicrVintIsActive?))))
          (if _output_get
            (bind _outactors_2 (Actor|GetAllActorswithInterface "/Game/CustomLogic/BP_Interferometer/BP_Komponenti/BPI_PhotodelCopyAssemble.BPI_PhotodelCopyAssemble_C"))
            (Class|BPIPhotodelCopyAssemble|OriginalAssembleComplete(Message) _outactors_2 (Math|Boolean|ANDBoolean (Variables|Default|GetStojkaIsActive?) (Variables|Default|GetZazhim1IsActive?) (Variables|Default|GetZazhim2IsActive?) (Variables|Default|GetLenseIsActive?) (Variables|Default|GetBolt1IsActive?) (Variables|Default|GetBolt2IsActive?) (Variables|Default|GetMicrVintIsActive?)))
            (Utilities|FlowControl|Delay 2.0)
            (CallFunction|AssembleCheck)
            (UserInterface|Viewport|AddtoViewport (Variables|Default|GetWidjet) 0)))))))

(event OnClicked(ТЗ_Стойка)
  (params (TouchedComponent :type Primitive%20Component%20Object%20Reference) (ButtonPressed :type Key%20Structure))
  (bind _cm_стойка (Variables|Default|GetCM_Стойка))
  (bind _relativelocation (Variables|/Script/Engine.SceneComponent|GetRelativeLocation _cm_стойка))
  (bind _outactors (Actor|GetAllActorsOfClasswithTag (Variables|Default|GetPhotodelPart) "1"))
  (if (Utilities|Array|IsValidIndex _outactors)
    (if (not (Variables|Default|GetStojkaIsActive?))
      (Variables|Default|SetStojkaIsActive? true)
      (Rendering|SetVisibility (Variables|Default|GetCM_Стойка) true false)
      (bind _z (Timeline|Stojka PlayFromStart)
        (:Update
          (Transformation|SetRelativeLocation _cm_стойка (Math|Vector|MakeVector (.x _relativelocation) (.y _relativelocation) _z) false true)
          (Development|PrintString "Стойка установлена")
          (bind _output_get (Variables|Default|SetAssembleComplite? (Math|Boolean|ANDBoolean (Variables|Default|GetStojkaIsActive?) (Variables|Default|GetZazhim1IsActive?) (Variables|Default|GetZazhim2IsActive?) (Variables|Default|GetLenseIsActive?) (Variables|Default|GetBolt1IsActive?) (Variables|Default|GetBolt2IsActive?) (Variables|Default|GetMicrVintIsActive?))))
          (if _output_get
            (bind _outactors_2 (Actor|GetAllActorswithInterface "/Game/CustomLogic/BP_Interferometer/BP_Komponenti/BPI_PhotodelCopyAssemble.BPI_PhotodelCopyAssemble_C"))
            (Class|BPIPhotodelCopyAssemble|OriginalAssembleComplete(Message) _outactors_2 (Math|Boolean|ANDBoolean (Variables|Default|GetStojkaIsActive?) (Variables|Default|GetZazhim1IsActive?) (Variables|Default|GetZazhim2IsActive?) (Variables|Default|GetLenseIsActive?) (Variables|Default|GetBolt1IsActive?) (Variables|Default|GetBolt2IsActive?) (Variables|Default|GetMicrVintIsActive?)))
            (Utilities|FlowControl|Delay 2.0)
            (CallFunction|AssembleCheck)
            (UserInterface|Viewport|AddtoViewport (Variables|Default|GetWidjet) 0)))))))

(event OnClicked(TZ_Vint2)
  (params (TouchedComponent :type Primitive%20Component%20Object%20Reference) (ButtonPressed :type Key%20Structure))
  (bind _cm_vint2 (Variables|Default|GetCM_Vint2))
  (bind _relativelocation (Variables|/Script/Engine.SceneComponent|GetRelativeLocation _cm_vint2))
  (bind _outactors (Actor|GetAllActorsOfClasswithTag (Variables|Default|GetPhotodelPart) "4"))
  (if (Utilities|Array|IsValidIndex _outactors)
    (if (not (Variables|Default|GetBolt2IsActive?))
      (Variables|Default|SetBolt2IsActive? true)
      (Rendering|SetVisibility (Variables|Default|GetCM_Vint2) true false)
      (bind (_direction _y _yrot) (Timeline|Vint2 PlayFromStart)
        (:Update
          (Transformation|SetRelativeLocationAndRotation _cm_vint2 (Math|Vector|MakeVector (.x _relativelocation) _y (.z _relativelocation)) (Math|Rotator|MakeRotator 0.0 _yrot 0.0) false false)
          (Development|PrintString "Винт 2 установлен")
          (bind _output_get (Variables|Default|SetAssembleComplite? (Math|Boolean|ANDBoolean (Variables|Default|GetStojkaIsActive?) (Variables|Default|GetZazhim1IsActive?) (Variables|Default|GetZazhim2IsActive?) (Variables|Default|GetLenseIsActive?) (Variables|Default|GetBolt1IsActive?) (Variables|Default|GetBolt2IsActive?) (Variables|Default|GetMicrVintIsActive?))))
          (if _output_get
            (bind _outactors_2 (Actor|GetAllActorswithInterface "/Game/CustomLogic/BP_Interferometer/BP_Komponenti/BPI_PhotodelCopyAssemble.BPI_PhotodelCopyAssemble_C"))
            (Class|BPIPhotodelCopyAssemble|OriginalAssembleComplete(Message) _outactors_2 (Math|Boolean|ANDBoolean (Variables|Default|GetStojkaIsActive?) (Variables|Default|GetZazhim1IsActive?) (Variables|Default|GetZazhim2IsActive?) (Variables|Default|GetLenseIsActive?) (Variables|Default|GetBolt1IsActive?) (Variables|Default|GetBolt2IsActive?) (Variables|Default|GetMicrVintIsActive?)))
            (Utilities|FlowControl|Delay 2.0)
            (CallFunction|AssembleCheck)
            (UserInterface|Viewport|AddtoViewport (Variables|Default|GetWidjet) 0)))))))

(event Custom|AssembleCheck
  (Development|PrintString "Сборка совершена" true true "(R=0.028321,G=1.000000,B=0.000000,A=1.000000)" 6.0))

(event EventBeginPlay
  (bind _returnvalue (UserInterface|CreateWidget "/Game/CustomLogic/BP_Interferometer/BP_Komponenti/Widjet_Assemble.Widjet_Assemble_C"))
  (Variables|Default|SetWidjet _returnvalue)
  (bind _outactors (Actor|GetAllActorsOfClass "BP_PhotodelBase_C"))
  (Variables|Default|SetBaseTransform (Transformation|GetWorldTransform (Variables|Default|GetDefaultSceneRoot)))
  (Development|PrintString "Hello")
  (Rendering|SetVisibility (Variables|Default|GetСМ_Зажим2) (Variables|BP_PhotodelBase_C|GetAssembleComplite? (Utilities|Array|Get(acopy) _outactors)) false)
  (Variables|Default|SetAssembleComplite? (Variables|BP_PhotodelBase_C|GetAssembleComplite? (Utilities|Array|Get(acopy) _outactors))))

(event Collision|EventActorBeginOverlap
  (params (OtherActor :type Actor%20Object%20Reference))
  (|CallParentFunction OtherActor) ; This node is disabled and will not be called.\nDrag off pins to build functionality.
)

(fn ConstructionScript
  (|CallParentFunction))

(fn KomponenttoAdd
  (params (ObjectIn :type Actor%20Object%20Reference))
  (Variables|Default|SetPhotodelPart (Utilities|GetClass ObjectIn))
  (return 0))

(fn AssembleState
  (params (AssembleStarted? :type Boolean) (AssembleEnded? :type Boolean))
  (bind _widjet (Variables|Default|GetWidjet))
  (bind _defaultsceneroot (Variables|Default|GetDefaultSceneRoot))
  (bind _widjet_2 (Variables|Default|GetWidjet))
  (bind _output_get (Variables|Default|SetAssemble%20Started? AssembleStarted?))
  (if _output_get
    (bind _outactors (Actor|GetAllActorsOfClass "/Game/PuzzleBP/Blueprints/PuzzlePlayerCharacter.PuzzlePlayerCharacter_C"))
    (bind _asplayer_controller (Utilities|Casting|CastToPlayerController (Pawn|GetController (Utilities|Array|Get(acopy) _outactors))))
    (Game|Player|SetViewTargetwithBlend _asplayer_controller (Variables|Default|GetCameraToSwitch) 1.0 "VTBlend_Cubic" 0.0 true)
    (Variables|Default|SetBaseTransform (Transformation|GetWorldTransform _defaultsceneroot))
    (Transformation|SetWorldTransform _defaultsceneroot (Math|Transform|MakeTransform "75.000000,-1070.000000,220.000000" "0,-60.000000,0.000000" "4.000000,4.000000,4.000000") false true)
    (if (UserInterface|Viewport|IsinViewport _widjet_2)
      (Widget|RemovefromParent _widjet_2))
    (else
      (bind _outactors_2 (Actor|GetAllActorsOfClass "/Game/PuzzleBP/Blueprints/PuzzlePlayerCharacter.PuzzlePlayerCharacter_C"))
      (bind _asplayer_controller_2 (Utilities|Casting|CastToPlayerController (Pawn|GetController (Utilities|Array|Get(acopy) _outactors_2))))
      (Game|Player|SetViewTargetwithBlend _asplayer_controller_2 (Variables|Default|GetStartingCamera) 1.0 "VTBlend_Cubic" 0.0 true)
      (Transformation|SetWorldTransform (Variables|Default|GetDefaultSceneRoot) (Variables|Default|GetBaseTransform) false true)
      (if (UserInterface|Viewport|IsinViewport _widjet)
        (Widget|RemovefromParent _widjet)))))

(fn OriginalAssembleComplete
  (params (OriginalAssembleComplite :type Boolean)))