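; BP_Mishen is a clickable interferometer part (by folder) that toggles the player's view between two cameras and shows or hides a slider widget.
; Clicking ObjectToSpawn finds the first PuzzlePlayerCharacter's controller and blends the view between StartingCamera and CameraToSwitch with a cubic blend.
; The same click creates the slider on first use, then toggles it in the viewport on later clicks.
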(event OnClicked(ObjectToSpawn)
  (params (TouchedComponent :type Primitive%20Component%20Object%20Reference) (ButtonPressed :type Key%20Structure))
  (bind _outactors (Actor|GetAllActorsOfClass "/Game/PuzzleBP/Blueprints/PuzzlePlayerCharacter.PuzzlePlayerCharacter_C"))
  (bind _asplayer_controller (Utilities|Casting|CastToPlayerController (Pawn|GetController (Utilities|Array|Get(acopy) _outactors))))
  (if (== (Variables|Default|GetCuurentCamera) (Variables|Default|GetStartingCamera))
    (Variables|Default|SetCuurentCamera (Variables|Default|GetCameraToSwitch))
    (else
      (Variables|Default|SetCuurentCamera (Variables|Default|GetStartingCamera))))
  (Game|Player|SetViewTargetwithBlend _asplayer_controller (Variables|Default|GetCuurentCamera) 1.0 "VTBlend_Cubic" 0.0 true)
  (if (Variables|Default|GetWidget)
    (if (UserInterface|Viewport|IsinViewport (stale _returnvalue))
      (Widget|RemovefromParent (stale _returnvalue))
      (else
        (UserInterface|Viewport|AddtoViewport (stale _returnvalue) 0)))
    (else
      (bind _returnvalue (UserInterface|CreateWidget "/Game/CustomLogic/BP_Interferometer/Slider.Slider_C"))
      (UserInterface|Viewport|AddtoViewport _returnvalue 0)
      (Variables|Default|SetWidget true))))

(event EventBeginPlay
  (Variables|Default|SetCuurentCamera (Variables|Default|GetStartingCamera)))

(fn ConstructionScript
  (|CallParentFunction))