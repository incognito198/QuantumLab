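; Actor for an interferometer assembly simulation, named as a photodetector or splitter part (Photodel), with most of its logic disconnected.
; BeginPlay hides the stand, clamp, micrometer screw, screw and lens meshes, and the S key saves and prints the current mirror angle.
; Unwired chains hold click selection with blue highlighting, part placement, mirror rotation and an angle slider tied to the InterferencePattern material collection.
; The other events are empty.
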(event OnClicked(TZ_Mirror)
  (params (TouchedComponent :type Primitive%20Component%20Object%20Reference) (ButtonPressed :type Key%20Structure)))

(event OnClicked(TZ_MicrScrew)
  (params (TouchedComponent :type Primitive%20Component%20Object%20Reference) (ButtonPressed :type Key%20Structure)))

(event OnClicked(SM_Стойка)
  (params (TouchedComponent :type Primitive%20Component%20Object%20Reference) (ButtonPressed :type Key%20Structure)))

(event Custom|Mirror)

(event Custom|Screw)

(event Custom|Assembled)

(event Custom|Unselect)

(event Custom|CurretntAngle
  (params (anle :type Float%20%28single-precision%29)))

(event Custom|MoveInterferometr
  (params (NewParam :type BP%20Socket%20Object%20Reference)))

(event EventBeginPlay
  (Rendering|SetVisibility (Variables|Default|GetСМ_стойка) false false))

(event Input|KeyboardEvents|S
  (params (Key :type Key%20Structure))
  (:Pressed
    (bind _output_get (Variables|Default|SetSavedAngle (Variables|Default|GetCurrentAngleMirror)))
    (Development|PrintString (Utilities|String|ToString(Float) _output_get))))

(fn ConstructionScript)

(fn Object
  (params (ObjectIn :type Actor%20Object%20Reference))
  (return 0))