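; BP_Inventory is a slot-based inventory that sizes its slot array (Слоты) to a configured count (КоличествоСлотов) on BeginPlay.
; Each slot holds an item class and a quantity, and a slot counts as empty when its class is invalid.
; Index-based queries report emptiness and quantity, while the item spec lookup from class defaults is unused.
; SearchEmptySlot is an unimplemented stub that always reports failure.
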(event EventBeginPlay
  (Utilities|Array|Resize (Variables|Default|GetСлоты) (Variables|Default|GetКоличествоСлотов)))

(fn ConstructionScript)

(fn IsSlotEmpty?
  (params (индекс :type Integer))
  (return (not (Utilities|IsValidClass (.ItemClass (Utilities|Struct|BreakStruct_InventorySlots (Utilities|Array|Get(acopy) (Variables|Default|GetСлоты) индекс)))))))

(fn GetItemInfoatIndex
  (params (индекс :type Integer))
  (bind _слоты (Variables|Default|GetСлоты))
  (bind _output (Utilities|Array|Get(acopy) _слоты индекс))
  (bind (_itemclass _количество) (Utilities|Struct|BreakStruct_InventorySlots _output))
  (if (Utilities|IsValidClass _itemclass)
    (return false "" _количество)
    (else
      (return true "" 0))))

(fn SearchEmptySlot
  (return false false))