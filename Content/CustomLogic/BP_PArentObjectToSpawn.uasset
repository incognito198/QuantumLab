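; BP_PArentObjectToSpawn is, by its name, a parent Blueprint for clickable spawnable objects in a puzzle game that go into the player's inventory.
; Clicking ObjectToSpawn passes itself to every actor implementing BPI_ChooseObject, then to every one implementing BPI_Photodelitel.
; It then prints its name and adds its ItemInfoStruct to the PuzzlePlayerCharacter's inventory.
; Its own interface functions are empty, and a PickUpItem branch never runs.
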(event OnClicked(ObjectToSpawn)
  (params (TouchedComponent :type Primitive%20Component%20Object%20Reference) (ButtonPressed :type Key%20Structure :default "None"))
  (bind _self self)
  (bind _outactors (Actor|GetAllActorswithInterface "/Game/CustomLogic/BPI_ChooseObject.BPI_ChooseObject_C"))
  (Class|BPIChooseObject|Object(Message) _outactors self)
  (bind _outactors_2 (Actor|GetAllActorswithInterface "/Game/CustomLogic/BP_Interferometer/BP_Komponenti/BPI_Photodelitel.BPI_Photodelitel_C"))
  (Class|BPIPhotodelitel|KomponenttoAdd(Message) _outactors_2 _self)
  (Development|PrintString (Utilities|GetObjectName _self))
  (bind _aspuzzle_player_character (Utilities|Casting|CastToPuzzlePlayerCharacter (Game|GetPlayerCharacter 0)))
  (Default|AddtoInventory (Variables|/Game/PuzzleBP/Blueprints/PuzzlePlayerCharacter.PuzzlePlayerCharacter_C|GetInventory _aspuzzle_player_character) (Variables|Default|GetItem%20Info%20Struct)))

(fn ConstructionScript)

(fn InetferometreAssembleState
  (return))

(fn KomponenttoAdd
  (params (ObjectIn :type Actor%20Object%20Reference))
  (return 0))

(fn Object
  (params (ObjectIn :type Actor%20Object%20Reference)))